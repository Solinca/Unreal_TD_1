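; BP_Cube is a test actor that recolours its cube mesh and animates its scale at runtime.
; On BeginPlay it creates a dynamic material instance from the mesh's first material and sets its BaseColor to a green tint.
; After a short delay a timeline drives the cube's world scale and restarts itself on finish to loop.
; An unconnected branch shows an alternative way to create and assign the dynamic material from MAT_CubeBase.
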(event EventBeginPlay
  (bind _cube (Variables|Default|GetCube))
  ;[0.15 0.15 0.15 0.5] Another Way
  (bind _returnvalue (Rendering|Material|CreateDynamicMaterialInstance _cube 0 (Rendering|Material|GetMaterial _cube 0) "None" :!class /Script/Engine.PrimitiveComponent))
  (Rendering|Material|SetVectorParameterValue _returnvalue "BaseColor" "(R=0.250014,G=1.000000,B=0.671572,A=1.000000)" :!class /Script/Engine.MaterialInstanceDynamic)
  (Utilities|FlowControl|Delay 2.0)
  (bind _value (Timeline|Timeline Play)
    (:Update
      (Transformation|SetWorldScale3D (Variables|Default|GetCube) (Math|Conversions|ToVector(Float) _value)))
    (:Finished
      (Timeline|Timeline PlayFromStart))))

(fn ConstructionScript)