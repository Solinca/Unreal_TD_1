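; Player character Blueprint that relays PlayerHealthComponent changes and handles death when health runs out.
; On BeginPlay it broadcasts current and max health to initialize the UI, then forwards each later health change through the same OnHealthChanged dispatcher.
; On depletion it ragdolls the mesh through physics simulation, signals the player controller to disable input and broadcasts OnHealthDepleted.
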(event OnHealthChanged(PlayerHealthComponent)
  (params (NewHealth :type Float%20%28single-precision%29) (MaxHealth :type Float%20%28single-precision%29))
  (Default|CallOnHealthChanged NewHealth MaxHealth))

(event OnHealthDepleted(PlayerHealthComponent)
  ;[0.15 0.15 0.15 0.5] Ragdoll
  (Physics|SetSimulatePhysics (Variables|Character|GetMesh) true)
  ;[0.15 0.15 0.15 0.5] Disable Input From PC_MyPlayerController
  (Default|CallDisableInputEvent)
  (Default|CallOnHealthDepleted))

(event EventBeginPlay
  ;[0.15 0.15 0.15 0.5] First On Health Call for UI
  (bind _returnvalue (Class|PlayerHealthComponent|GetHealth (Variables|Default|GetPlayerHealthComponent)))
  (bind _returnvalue_2 (Class|PlayerHealthComponent|GetMaxHealth (Variables|Default|GetPlayerHealthComponent)))
  (Default|CallOnHealthChanged _returnvalue _returnvalue_2))

(fn ConstructionScript)