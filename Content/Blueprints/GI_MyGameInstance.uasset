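; Game instance scaffold for saving and loading an SG_MySaveGame object in a single slot, held in CustomSave.
; It sketches blocking and async variants, with loading creating a new save if none exists and async paths calling done notifications.
; The AsyncSave and AsyncLoad events are empty and every save/load chain is disconnected, so none of it runs.
; The async save chain includes a delay to simulate lag.
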(event Custom|AsyncLoad
  ;[0.15 0.15 0.15 0.5] Async Load
)

(event Custom|AsyncSave
  ;[0.15 0.15 0.15 0.5] Async Save
)